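; BP_ProjectileVFXSpawner is a placeable actor that repeatedly fires projectiles to display projectile VFX sets.
; On BeginPlay a looping timer spawns a BP_ProjectileMaster at the spawner's transform every launch interval.
; Each spawned projectile receives the spawner's muzzle, trail and impact effects plus destroy delay, and its movement velocity is set along the spawner's forward vector at the configured speed.
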(event Custom|SpawnProjectileVFX
  (bind _returnvalue (Game|SpawnActorfromClass "/Game/Projectile_Assets/BP/BP_ProjectileMaster.BP_ProjectileMaster_C" (Transformation|GetActorTransform) "Undefined" "MultiplyWithRoot" 0 0))
  (bind _output_get (Variables|Default|SetSpawnedProjectile _returnvalue))
  (Utilities|IsValid _output_get
    (:Is%20Valid
      (Utilities|FlowControl|Sequence
        (:then_0
          (Variables|/Game/Projectile_Assets/BP/BP_ProjectileMaster.BP_ProjectileMaster_C|SetMuzzleVFX (Variables|Default|GetSpawnedProjectile) (Variables|Default|GetMuzzleVFX))
          (Variables|/Game/Projectile_Assets/BP/BP_ProjectileMaster.BP_ProjectileMaster_C|SetHitImpactVFX (Variables|Default|GetSpawnedProjectile) (Variables|Default|GetHitImpactVFX))
          (Class|NiagaraComponent|SetAsset (Variables|/Game/Projectile_Assets/BP/BP_ProjectileMaster.BP_ProjectileMaster_C|GetProjectileVFXComponent (Variables|Default|GetSpawnedProjectile)) (Variables|Default|GetProjectileVFX) true)
          (Variables|/Game/Projectile_Assets/BP/BP_ProjectileMaster.BP_ProjectileMaster_C|SetProjectileDestroyDelay (Variables|Default|GetSpawnedProjectile) (Variables|Default|GetProjectileDestroyDelay)))
        (:then_1
          (Variables|/Script/Engine.MovementComponent|SetVelocity (Variables|/Game/Projectile_Assets/BP/BP_ProjectileMaster.BP_ProjectileMaster_C|GetProjectileVFXMovementComponent (Variables|Default|GetSpawnedProjectile)) (* (Transformation|GetActorForwardVector) (Variables|Default|GetProjectileSpeed))))))))

(event EventBeginPlay
  (Utilities|Time|SetTimerbyEvent (delegate Custom|SpawnProjectileVFX) (Variables|Default|GetProjectileLaucnhInterval) true))

(fn ConstructionScript)