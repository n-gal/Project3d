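; Master projectile actor that plays Niagara effects over its lifetime, from muzzle to impact.
; On BeginPlay it spawns the muzzle effect at its own location.
; When the box collider overlaps a BlockingVolume, it stops movement, sets the KillParticle variable on the projectile effect, spawns the impact effect and destroys itself after a delay.
; Other overlapped actors are ignored, and no damage is applied.
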(event OnComponentBeginOverlap(ProjectileBoxCollider)
  (params (OverlappedComponent :type Primitive%20Component%20Object%20Reference) (OtherActor :type Actor%20Object%20Reference) (OtherComp :type Primitive%20Component%20Object%20Reference) (OtherBodyIndex :type Integer) (bFromSweep :type Boolean) (SweepResult :type Hit%20Result%20Structure%20%28by%20ref%29))
  (Utilities|Casting|CastToBlockingVolume OtherActor)
  (Components|Movement|StopMovementImmediately (Variables|Default|GetProjectileVFXMovementComponent))
  (Class|NiagaraComponent|SetVariableBool (Variables|Default|GetProjectileVFXComponent) "KillParticle" true)
  (CallFunction|SpawnVFX (Variables|Default|GetHitImpactVFX))
  (Utilities|FlowControl|Delay (Variables|Default|GetProjectileDestroyDelay))
  (Actor|DestroyActor))

(event EventBeginPlay
  (CallFunction|SpawnVFX (Variables|Default|GetMuzzleVFX)))

(event Collision|EventActorBeginOverlap
  (params (OtherActor :type Actor%20Object%20Reference)))

(event EventTick
  (params (DeltaSeconds :type Float%20%28single-precision%29)))

(fn ConstructionScript)

(fn SpawnVFX
  (params (VFX :type Niagara%20System%20Object%20Reference))
  (Utilities|IsValid VFX
    (:Is%20Valid
      (Niagara|SpawnSystematLocation VFX (Transformation|GetActorLocation)))))