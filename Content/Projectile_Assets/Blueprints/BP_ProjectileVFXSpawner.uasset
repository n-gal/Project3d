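; Spawner actor that fires BP_ProjectileMaster projectiles from its own transform with configurable VFX.
; It spawns one on BeginPlay and sets a timer to call the spawn event again after ProjectileGap.
; Each spawned projectile receives the muzzle, main Niagara and impact effects plus a destroy delay.
; Its movement component velocity is then set along the spawner's forward vector, scaled by ProjectileSpeed.
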(event Custom|SpawnProjectileVFX
  (bind _returnvalue (Game|SpawnActorfromClass "/Game/Projectile_Assets/Blueprints/BP_ProjectileMaster.BP_ProjectileMaster_C" (Transformation|GetActorTransform) "Undefined" "MultiplyWithRoot" 0 0))
  (bind _output_get (Variables|Default|SetSpawnedProjectile _returnvalue))
  (Utilities|IsValid _output_get
    (:Is%20Valid
      (Utilities|FlowControl|Sequence
        (:then_0
          (Variables|/Game/Projectile_Assets/Blueprints/BP_ProjectileMaster.BP_ProjectileMaster_C|SetMuzzleVFX (Variables|Default|GetSpawnedProjectile) (Variables|Default|GetMuzzle%20VFX))
          (Class|NiagaraComponent|SetAsset (Variables|/Game/Projectile_Assets/Blueprints/BP_ProjectileMaster.BP_ProjectileMaster_C|GetProjectileVFX_Component (Variables|Default|GetSpawnedProjectile)) (Variables|Default|GetMainProjectileVFX) true)
          (Variables|/Game/Projectile_Assets/Blueprints/BP_ProjectileMaster.BP_ProjectileMaster_C|SetHItImpactVFX (Variables|Default|GetSpawnedProjectile) (Variables|Default|GetHIt%20Impact%20VFX))
          (Class|NiagaraComponent|SetAsset (Variables|/Game/Projectile_Assets/Blueprints/BP_ProjectileMaster.BP_ProjectileMaster_C|GetProjectileVFX_Component (Variables|Default|GetSpawnedProjectile)) (Variables|Default|GetMainProjectileVFX) true)
          (Variables|/Game/Projectile_Assets/Blueprints/BP_ProjectileMaster.BP_ProjectileMaster_C|SetProjectileDestroy_Delay (Variables|Default|GetSpawnedProjectile) (Variables|Default|GetProjectileDestroyDelay)))
        (:then_1
          (Variables|/Script/Engine.MovementComponent|SetVelocity (Variables|/Game/Projectile_Assets/Blueprints/BP_ProjectileMaster.BP_ProjectileMaster_C|GetProjectileVFX_Movement (Variables|Default|GetSpawnedProjectile)) (* (Variables|Default|GetProjectileSpeed) (Transformation|GetActorForwardVector))))))))

(event EventBeginPlay
  (CallFunction|SpawnProjectileVFX)
  (Utilities|Time|SetTimerbyEvent (delegate Custom|SpawnProjectileVFX) (Variables|Default|GetProjectileGap)))

(fn ConstructionScript)