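; BP_ProjectileMaster is a base projectile actor that handles muzzle, flight and impact VFX.
; On BeginPlay it spawns the muzzle effect through SpawnVFX, a helper that validity-checks a system and spawns it at the actor's location.
; Box overlaps react only to Blocking Volumes: movement stops, a "Kill Particles" variable is set on the projectile VFX, the impact effect spawns, and the actor self-destroys after a configurable delay.
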(event OnComponentBeginOverlap(Projectile_BoxCollision)
  (params (OverlappedComponent :type Primitive%20Component%20Object%20Reference) (OtherActor :type Actor%20Object%20Reference) (OtherComp :type Primitive%20Component%20Object%20Reference) (OtherBodyIndex :type Integer) (bFromSweep :type Boolean) (SweepResult :type Hit%20Result%20Structure%20%28by%20ref%29))
  ;[0.15 0.15 0.15 0.5] Collision
  (Utilities|Casting|CastToBlockingVolume OtherActor)
  ;[0.15 0.15 0.15 0.5] Stop Projectile movement
  (Components|Movement|StopMovementImmediately (Variables|Default|GetProjectileVFX_Movement))
  (Class|NiagaraComponent|SetVariableBool (Variables|Default|GetProjectileVFX_Component) "Kill Particles" true)
  (CallFunction|SpawnVFX (Variables|Default|GetHItImpactVFX))
  (Utilities|FlowControl|Delay (Variables|Default|GetProjectileDestroy_Delay))
  (Actor|DestroyActor))

(event EventBeginPlay
  ;[0.15 0.15 0.15 0.5] Muzzle
  (CallFunction|SpawnVFX (Variables|Default|GetMuzzleVFX)))

(fn ConstructionScript)

(fn SpawnVFX
  (params (VFXToSpawn :type Niagara%20System%20Object%20Reference))
  (Utilities|IsValid VFXToSpawn
    (:Is%20Valid
      (Niagara|SpawnSystematLocation VFXToSpawn (Transformation|GetActorLocation)))))